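; Player controller Blueprint for a tank that manages the player's HUD and death screen.
; When FoundAimingComponent fires, it creates the PlayerUI widget, hands it the aiming component reference and adds it to the viewport.
; Each Tick it checks CallDeathScreen and, when true, shows a DeathScreen widget, enables the mouse cursor and pauses the game.
; It disables ticking while paused, so the pause also halts that check.
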(event EventFoundAimingComponent
  (params (AimCompRef :type Tank%20Aiming%20Component%20Object%20Reference))
  (bind _returnvalue (UserInterface|CreateWidget "/Game/UI/PlayerUI.PlayerUI_C"))
  (Variables|/Game/UI/PlayerUI.PlayerUI_C|SetBP_Aiming_Comp_Reference%20 _returnvalue AimCompRef)
  (UserInterface|Viewport|AddtoViewport _returnvalue 0))

(event EventTick
  (params (DeltaSeconds :type Float%20%28single-precision%29))
  (Class|Actor|SetTickablewhenPaused false)
  (bind _returnvalue (Class|TankPlayerController|CallDeathScreen false))
  (if _returnvalue
    (bind _returnvalue_2 (UserInterface|CreateWidget "/Game/UI/DeathScreen.DeathScreen_C"))
    (UserInterface|Viewport|AddtoViewport _returnvalue_2 0)
    (Variables|Default|SetbShowMouseCursor true)
    (Game|SetGamePaused true)))

(fn ConstructionScript)